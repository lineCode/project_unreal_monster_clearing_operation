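; BP_Water is a test actor that applies a gameplay effect to characters touching its box volume.
; On any actor begin overlap, it loops over everything inside Box and casts each to MCOCharacter.
; Each character with a valid ability system component applies OnPickupEffect to itself, so characters already inside receive it again on each new overlap.
; The actor neither removes the effect nor destroys itself.
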(event EventBeginPlay)

(event Collision|EventActorBeginOverlap
  (params (OtherActor :type Actor%20Object%20Reference))
  (for _array_element (Collision|GetOverlappingActors (Variables|Default|GetBox) 0 :!class /Script/Engine.PrimitiveComponent)
    (bind _asmcocharacter (Utilities|Casting|CastToMCOCharacter _array_element))
    (if (Utilities|IsValid (Ability|GetAbilitySystemComponent _asmcocharacter))
      (GameplayEffects|ApplyGameplayEffectSpecToSelf (Ability|GetAbilitySystemComponent _asmcocharacter) (GameplayEffects|MakeOutgoingSpec (Ability|GetAbilitySystemComponent _asmcocharacter) (Variables|Default|GetOnPickupEffect) 0.0 (GameplayEffects|MakeEffectContext (Ability|GetAbilitySystemComponent _asmcocharacter)))))))

(event EventTick
  (params (DeltaSeconds :type Float%20%28single-precision%29)))

(fn ConstructionScript)